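; BP_Spawner continuously lays down a descending track of ground pieces, drawing each from its ACObjectPool component.
; BeginPlay spawns two initial pieces, then a looping timer adds another at a fixed forward and downward step.
; A NextRandomGround countdown varies the layout: at zero a piece gets a random lateral position and the counter rerolls; otherwise pieces align with the first spawn's Y.
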(event `self.ReceiveBeginPlay`
  (bind _nextspawnlocation (`self.nextSpawnLocation`))
  (`/Game/Core/GameplaySystems/ObjectPool/AC_ObjectPool.SpawnFromPool` (`self.AC_ObjectPool`) (`self.firstSpawnLocation`))
  (set `self.nextSpawnLocation` (`KismetMathLibrary.MakeTransform` (`KismetMathLibrary.MakeVector` (+ (.x (.location _nextspawnlocation)) 1860.0) (.y (.location (`self.firstSpawnLocation`))) (+ (.z (.location _nextspawnlocation)) -677.0)) (.rotation _nextspawnlocation) (.scale _nextspawnlocation)))
  (`/Game/Core/GameplaySystems/ObjectPool/AC_ObjectPool.SpawnFromPool` (`self.AC_ObjectPool`) (`self.nextSpawnLocation`))
  (`KismetSystemLibrary.K2_SetTimerDelegate` (delegate `groundSpawner`) 1.2 true))

(event `groundSpawner`
  (bind _nextspawnlocation (`self.nextSpawnLocation`))
  (bind _nextspawnlocation_2 (`self.nextSpawnLocation`))
  (if (== (`self.nextRandomGround`) 0)
    (set `self.nextSpawnLocation` (`KismetMathLibrary.MakeTransform` (`KismetMathLibrary.MakeVector` (+ (.x (.location _nextspawnlocation_2)) 1860.0) (`KismetMathLibrary.RandomFloatInRange` -2070.0 1500.0) (+ (.z (.location _nextspawnlocation_2)) -677.0)) (.rotation _nextspawnlocation_2) (.scale _nextspawnlocation_2)))
    (`/Game/Core/GameplaySystems/ObjectPool/AC_ObjectPool.SpawnFromPool` (`self.AC_ObjectPool`) (`self.nextSpawnLocation`))
    (set `self.nextRandomGround` (`KismetMathLibrary.RandomInteger` 3))
    (else
      (set `self.nextSpawnLocation` (`KismetMathLibrary.MakeTransform` (`KismetMathLibrary.MakeVector` (+ (.x (.location _nextspawnlocation)) 1860.0) (.y (.location (`self.firstSpawnLocation`))) (+ (.z (.location _nextspawnlocation)) -677.0)) (.rotation _nextspawnlocation) (.scale _nextspawnlocation)))
      (`/Game/Core/GameplaySystems/ObjectPool/AC_ObjectPool.SpawnFromPool` (`self.AC_ObjectPool`) (`self.nextSpawnLocation`))
      (bind _result (`/Engine/EditorBlueprintResources/StandardMacros.DecrementInt` (`self.nextRandomGround`))
        (:`  `
          (set `self.nextRandomGround` _result))))))

(fn `UserConstructionScript`)