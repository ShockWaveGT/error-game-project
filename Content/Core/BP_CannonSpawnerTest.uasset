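; BP_CannonSpawnerTest is a test actor that periodically spawns a cannon from its ACObjectPool component.
; BeginPlay starts SpawnTester, which picks one of two hardcoded spawn transforms depending on whether the current level is "Menu".
; Each branch spawns from the pool, prints a debug message, then re-calls SpawnTester after a one-minute Delay, forming an endless loop.
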(event `self.ReceiveBeginPlay`
  (`self.SpawnTester`))

(event `SpawnTester`
  (bind _returnvalue (`GameplayStatics.GetCurrentLevelName` true))
  (if (`KismetStringLibrary.EqualEqual_StrStr` _returnvalue "Menu")
    (`/Game/Core/GameplaySystems/ObjectPool/AC_ObjectPool.SpawnFromPool` (`self.AC_ObjectPool`) (`KismetMathLibrary.MakeTransform` (230.0 -620.0 110.0)))
    (`KismetSystemLibrary.PrintString` "Spawned Cannon|15sec live(BP_CannonSpawnerTest)" true true (struct :`G` 0.66 :`B` 1.0 :`A` 1.0) 15.0)
    (`KismetSystemLibrary.Delay` 60.0)
    (`self.SpawnTester`)
    (else
      (`/Game/Core/GameplaySystems/ObjectPool/AC_ObjectPool.SpawnFromPool` (`self.AC_ObjectPool`) (`KismetMathLibrary.MakeTransform` (220.0 110.0 180.0)))
      (`KismetSystemLibrary.PrintString` "Spawned Cannon|15sec live(BP_CannonSpawnerTest)" true true (struct :`G` 0.66 :`B` 1.0 :`A` 1.0) 15.0)
      (`KismetSystemLibrary.Delay` 60.0)
      (`self.SpawnTester`))))

(fn `UserConstructionScript`)