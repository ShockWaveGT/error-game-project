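; Base pooled actor for the object pool system, toggled between active and dormant instead of spawned and destroyed.
; SetInUse switches collision, visibility and tick together, and BeginPlay starts the actor dormant.
; Activation restarts a one-shot TimeToLive timer that calls ReturnToPool, which sets the actor back to not in use.
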(event `self.ReceiveBeginPlay`
  (`self.SetInUse` false))

(event `SetInUse`
  (params (InUse :type Boolean))
  (set `self.InUse` InUse)
  (`self.SetActorEnableCollision` InUse)
  (`self.SetActorHiddenInGame` (not InUse))
  (`self.SetActorTickEnabled` InUse)
  (`KismetSystemLibrary.K2_ClearAndInvalidateTimerHandle` (`self.TimeToLiveTmp`))
  (if InUse
    (bind _returnvalue (`KismetSystemLibrary.K2_SetTimerDelegate` (delegate `ReturnToPool`) (`self.TimeToLive`)))
    (set `self.TimeToLiveTmp` _returnvalue)))

(event `ReturnToPool`
  (`self.SetInUse` false))

(fn `UserConstructionScript`)