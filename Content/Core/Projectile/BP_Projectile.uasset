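; BP_Projectile is a reusable projectile, toggled by an in-use state, that launches its BeachSK component forward when activated.
; SetinUse calls the parent implementation, then applies a forward velocity-change impulse to BeachSK.
; After a fixed delay it sets itself out of use, which suggests object pooling.
; BeginPlay, overlap and Tick are empty, so the Blueprint itself has no hit handling.
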(event `self.ReceiveBeginPlay`)

(event `self.ReceiveActorBeginOverlap`
  (params (OtherActor :type "Actor Object Reference")))

(event `self.SetInUse`
  (params (InUse :type Boolean))
  (`parent.SetInUse` InUse)
  (if InUse
    (`PrimitiveComponent.AddImpulse` (`self.BeachSK`) (* (`self.GetActorForwardVector`) 3000.0) "None" true)
    ;[1 1 1] Overlap reminder
    (`KismetSystemLibrary.Delay` 10.0)
    (`self.SetInUse` false)))

(fn `UserConstructionScript`)